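; BP_PUp_SlowLog is a spinning power-up pickup that slows the spike log in the side-scroller.
; Tick rotates the cone mesh, and when the player character overlaps the box it calls SlowSpeed on the first SpikeLog found, then destroys itself.
; A ReturnToRegularSpeed event, marked as a first attempt and not called here, recomputes the game mode's log speed after a short delay and applies it to the log.
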(event `self.ReceiveTick`
  (params (DeltaSeconds :type "Float (single-precision)"))
  ;[1 1 1] Rotación
  (`SceneComponent.K2_AddWorldRotation` (`self.Cone`) (struct :`Yaw` 0.75) false false))

(event `self.Box.OnComponentBeginOverlap`
  (params (OverlappedComponent :type "PrimitiveComponent Object Reference") (OtherActor :type "Actor Object Reference") (OtherComp :type "PrimitiveComponent Object Reference") (OtherBodyIndex :type Integer) (bFromSweep :type Boolean) (SweepResult :type "HitResult Structure (by ref)"))
  (cast `/Game/SideScrollerBP/Blueprints/OGSideScrollerCharacter` OtherActor)
  (bind _outactors (`GameplayStatics.GetAllActorsOfClass` "/Game/RISE/LvlGenrating/SpikeLog.SpikeLog_C"))
  (`/Game/RISE/LvlGenrating/SpikeLog.SlowSpeed` (`|GetArrayItem` _outactors))
  (`self.K2_DestroyActor`))

(event `ReturnToRegularSpeed`
  ;[1 1 1] intento uno
  (bind _asogside_scroller_game_mode (cast `/Game/RISE/OGSideScrollerGameMode` (`GameplayStatics.GetGameMode`)))
  (`KismetSystemLibrary.Delay` 0.2)
  (bind _output_get (set `/Game/RISE/OGSideScrollerGameMode.CurrentLogSpeed` (+ (`/Game/RISE/OGSideScrollerGameMode.SlowLog` _asogside_scroller_game_mode) (`/Game/RISE/OGSideScrollerGameMode.PUpLogSpeed` _asogside_scroller_game_mode)) _asogside_scroller_game_mode))
  (bind _outactors (`GameplayStatics.GetAllActorsOfClass` "/Game/RISE/LvlGenrating/SpikeLog.SpikeLog_C"))
  (set `/Game/RISE/LvlGenrating/SpikeLog.SpeedUp` (`KismetMathLibrary.MakeVector` 0.0 0.0 _output_get) (`|GetArrayItem` _outactors)))

(fn `UserConstructionScript`)