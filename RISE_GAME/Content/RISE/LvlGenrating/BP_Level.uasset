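; Level segment for a vertical side-scroller that builds one floor of the climb, marked buggy in its graph.
; On BeginPlay it fills fixed positions with Floor actors, leaving random gaps as BP_EmptyFloorCollision, and spawns a random power-up when the player's score matches the GameMode counter.
; One-shot triggers ask the GameMode to add a level and raise the player's score while speeding up the SpikeLog.
; GetAttachTransform exposes the AttachPoint transform.
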(event `self.ReceiveBeginPlay`
  (bind _randomint3 (`self.RandomInt3`))
  (bind _randomint2 (`self.RandomInt2`))
  ;[1 1 1] Buggy!!!!
  (set `self.GenerarEspacios` (`KismetMathLibrary.RandomIntegerInRange` 0 10))
  (set `self.RandomInt1` (`KismetMathLibrary.RandomIntegerInRange` 0 3))
  (set `self.RandomInt2` (`KismetMathLibrary.RandomIntegerInRange` 3 7))
  (set `self.RandomInt3` (`KismetMathLibrary.RandomIntegerInRange` 7 10))
  ;;[1 1 1] Generate 1 space
  (if (< (`self.GenerarEspacios`) 5)
    (set `self.RandomInt2` _randomint3)
    (set `self.RandomInt1` _randomint3)
    (bind _output_get (set `self.Position` (`|MakeArray` (`self.FloorPos8`) (`self.FloorPos7`) (`self.FloorPos6`) (`self.FloorPos5`) (`self.FloorPos4`) (`self.FloorPos3`) (`self.FloorPos2`) (`self.FloorPos1`) (`self.FloorPos9`) (`self.FloorPos10`) (`self.FloorPos11`)) :!label _label))
    (for (_ _array_index) _output_get
      (if (or (== _array_index (`self.RandomInt1`)) (== _array_index (`self.RandomInt2`)) (== _array_index (`self.RandomInt3`)))
        (if (or (and (== (`self.RandomInt1`) 3) (== _randomint2 4)) (and (== _randomint2 7) (== (`self.RandomInt3`) 8)))
          (bind _returnvalue (`SceneComponent.K2_GetComponentLocation` (`|GetArrayItem` (`self.Position`) _array_index)))
          (`|SpawnActorFromClass` "/Game/RISE/LvlGenrating/Floor.Floor_C" (`KismetMathLibrary.MakeTransform` _returnvalue) "Undefined" "OverrideRootScale" null null :!label _label_2)
          (else
            (`|SpawnActorFromClass` "/Game/RISE/LvlGenrating/BP_EmptyFloorCollision.BP_EmptyFloorCollision_C" (`KismetMathLibrary.MakeTransform` _returnvalue (struct)) "Undefined" "OverrideRootScale" null null)))
        (else
          (goto _label_2))))
    ;[1 1 1] Si el PowerUp == Puntos, genera un powerup
    (bind _asogside_scroller_character (cast `/Game/SideScrollerBP/Blueprints/OGSideScrollerCharacter` (`GameplayStatics.GetPlayerCharacter` 0)))
    (bind _asogside_scroller_game_mode (cast `/Game/RISE/OGSideScrollerGameMode` (`GameplayStatics.GetGameMode`)))
    (if (== (`/Game/SideScrollerBP/Blueprints/OGSideScrollerCharacter.PointScore` _asogside_scroller_character) (`/Game/RISE/OGSideScrollerGameMode.NextPowerUpCounter` _asogside_scroller_game_mode))
      (`self.PowerUp`))
    (else
      ;;[1 1 1] Generate 2
      (if (< (`self.GenerarEspacios`) 9)
        (set `self.RandomInt1` (`self.RandomInt3`))
        (goto _label)
        (else
          ;;[1 1 1] Generate 3
          (if (>= (`self.GenerarEspacios`) 9)
            (goto _label)))))))

(event `self.EndLevel.OnComponentBeginOverlap`
  (params (OverlappedComponent :type "PrimitiveComponent Object Reference") (OtherActor :type "Actor Object Reference") (OtherComp :type "PrimitiveComponent Object Reference") (OtherBodyIndex :type Integer) (bFromSweep :type Boolean) (SweepResult :type "HitResult Structure (by ref)"))
  ;[0.3783 0.09705 1] Cada vez que sube una plataforma, genera un piso adicional encima del ultimo creado
  (`/Engine/EditorBlueprintResources/StandardMacros.DoOnce` false
    (:`Completed`
      (bind _asogside_scroller_game_mode (cast `/Game/RISE/OGSideScrollerGameMode` (`GameplayStatics.GetGameMode`)))
      (`/Game/RISE/OGSideScrollerGameMode.AddLevel` _asogside_scroller_game_mode))))

(event `PowerUp`
  ;[0.3783 0.09705 1] Esponea camara power up despues del 5to piso random
  (bind _asogside_scroller_game_mode (cast `/Game/RISE/OGSideScrollerGameMode` (`GameplayStatics.GetGameMode`)))
  ;;[1 1 1] Juega las probabilidades en cual pueda aparecer el powerup
  (`/Game/RISE/OGSideScrollerGameMode.NxtPowerUp` _asogside_scroller_game_mode)
  (bind _output_get (set `/Game/RISE/OGSideScrollerGameMode.PwrUpPositionProbability` (`KismetMathLibrary.RandomIntegerInRange` 1 1) (stale `self.ReceiveBeginPlay` _asogside_scroller_game_mode)))
  (bind _output_get_2 (set `/Game/RISE/OGSideScrollerGameMode.PowerUpPosEnPiso` (`KismetMathLibrary.RandomIntegerInRange` 1 1) (stale `self.ReceiveBeginPlay` _asogside_scroller_game_mode)))
  (if (== _output_get_2 _output_get)
    (`/Game/RISE/OGSideScrollerGameMode.NotificationOfPowerUP` _asogside_scroller_game_mode)
    (bind _output_get_3 (set `self.PowerUps` (`|MakeArray` (`self.PowerUpPos1`) (`self.PowerUpPos2`) (`self.PowerUpPos3`))))
    ;;[1 1 1] Si PUPEP es igual al index, genera la posicion en la posicion que es igual. Si no es igual, no genera nada.
    (for (_ _array_index) _output_get_3
      (if (== _array_index (`/Game/RISE/OGSideScrollerGameMode.PowerUpPosEnPiso` (stale `self.ReceiveBeginPlay` _asogside_scroller_game_mode)))
        (`|SpawnActorFromClass` (`|GetArrayItem` (`self.PowerUpList`) (`KismetMathLibrary.RandomIntegerInRange` 0 1)) (`KismetMathLibrary.MakeTransform` (`SceneComponent.K2_GetComponentLocation` (`|GetArrayItem` (`self.PowerUps`) _array_index))) "Undefined" "OverrideRootScale" null null)))))

(event `self.Point.OnComponentBeginOverlap`
  (params (OverlappedComponent :type "PrimitiveComponent Object Reference") (OtherActor :type "Actor Object Reference") (OtherComp :type "PrimitiveComponent Object Reference") (OtherBodyIndex :type Integer) (bFromSweep :type Boolean) (SweepResult :type "HitResult Structure (by ref)"))
  ;[0.3783 0.09705 1] Cuenta el level más alto llegado y aumenta velocidad
  (`/Engine/EditorBlueprintResources/StandardMacros.DoOnce` false
    (:`Completed`
      (bind _asogside_scroller_character (cast `/Game/SideScrollerBP/Blueprints/OGSideScrollerCharacter` OtherActor))
      (`/Engine/EditorBlueprintResources/StandardMacros.IncrementInt` (`/Game/SideScrollerBP/Blueprints/OGSideScrollerCharacter.PointScore` _asogside_scroller_character)
        (:`  `
          (bind _outactors (`GameplayStatics.GetAllActorsOfClass` "/Game/RISE/LvlGenrating/SpikeLog.SpikeLog_C"))
          (`/Game/RISE/LvlGenrating/SpikeLog.Speed` (`|GetArrayItem` _outactors)))))))

(fn `GetAttachTransform`
  (returns (NewParam :type "Transform Structure"))
  ;[0.3783 0.09705 1] Consigue la localidad del AttachPoint
  (return (`SceneComponent.K2_GetComponentToWorld` (`self.AttachPoint`))))

(fn `NewPowerUp`)

(fn `UserConstructionScript`)