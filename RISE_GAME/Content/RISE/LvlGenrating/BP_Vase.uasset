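; BP_Vase is a breakable vase that the side-scroller player destroys by dashing into it, earning 3 points.
; On collision begin overlap it casts to OGSideScrollerCharacter, checks IsDashing, adds to that character's RealScore and destroys itself.
; The dash is only checked when overlap begins, so starting a dash while already overlapping leaves the vase intact, as a FIX comment notes.
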(event `self.ReceiveActorBeginOverlap`
  (params (OtherActor :type "Actor Object Reference")))

(event `self.ReceiveTick`
  (params (DeltaSeconds :type "Float (single-precision)")))

(event `self.VaseCollision.OnComponentBeginOverlap`
  (params (OverlappedComponent :type "PrimitiveComponent Object Reference") (OtherActor :type "Actor Object Reference") (OtherComp :type "PrimitiveComponent Object Reference") (OtherBodyIndex :type Integer) (bFromSweep :type Boolean) (SweepResult :type "HitResult Structure (by ref)"))
  ;[1 1 1] Lo que destruye el vase cuando el player está overlapping y dashing.
  ; *** FIX: Jarrón no se destruye cuando se activa el dash mientras esté overlapping; solo destruye si hace overlap durante el dash.
  (bind _asogside_scroller_character (cast `/Game/SideScrollerBP/Blueprints/OGSideScrollerCharacter` OtherActor))
  (bind _output_get (set `self.IsOVerlapping` true))
  (if (and _output_get (`/Game/SideScrollerBP/Blueprints/OGSideScrollerCharacter.IsDashing` _asogside_scroller_character))
    (set `/Game/SideScrollerBP/Blueprints/OGSideScrollerCharacter.RealScore` (+ (`/Game/SideScrollerBP/Blueprints/OGSideScrollerCharacter.RealScore` _asogside_scroller_character) 3) _asogside_scroller_character)
    (`self.K2_DestroyActor`)))

(event `self.VaseCollision.OnComponentEndOverlap`
  (params (OverlappedComponent :type "PrimitiveComponent Object Reference") (OtherActor :type "Actor Object Reference") (OtherComp :type "PrimitiveComponent Object Reference") (OtherBodyIndex :type Integer))
  ;[1 1 1] Lo que destruye el vase cuando el player está overlapping y dashing.
  ; *** FIX: Jarrón no se destruye cuando se activa el dash mientras esté overlapping; solo destruye si hace overlap durante el dash.
  (cast `/Game/SideScrollerBP/Blueprints/OGSideScrollerCharacter` OtherActor)
  (set `self.IsOVerlapping` false))

(fn `UserConstructionScript`)